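; Player pawn for a Blueprint tutorial that moves sideways from Enhanced Input.
; BeginPlay adds the tutorial mapping context to the first player controller's subsystem, then makes a zero-length swept offset with no displacement.
; The move action feeds its X value into movement input along the control rotation's right vector; there is no forward movement.
; Tick is disabled, and leftover print and movement nodes never run.
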(event Input|EnhancedActionEvents|EnhancedInputActionIA_MoveArroundBlueprintTutorial
  (params (ActionValue :type Vector%202D%20Structure) (ElapsedSeconds :type Float%20%28double-precision%29) (TriggeredSeconds :type Float%20%28double-precision%29) (InputAction :type Input%20Action%20Object%20Reference :default "/Game/Inputs/BlueprintTutorial/IA_MoveArroundBlueprintTutorial.IA_MoveArroundBlueprintTutorial"))
  (Pawn|Input|AddMovementInput (Math|Vector|GetRightVector (Pawn|GetControlRotation :!class /Script/Engine.Pawn)) (.x ActionValue) false))

(event EventBeginPlay
  (bind _returnvalue (Game|GetPlayerController 0))
  (bind _returnvalue_2 (PlayerController|LocalPlayerSubsystems|GetEnhancedInputLocalPlayerSubsystem _returnvalue))
  (Utilities|IsValid _returnvalue_2
    (:Is%20Valid
      (Input|AddMappingContext _returnvalue_2 "/Game/Inputs/BlueprintTutorial/IMC_BlueprintTutorial.IMC_BlueprintTutorial" 0 "(bIgnoreAllPressedKeysUntilRelease=True,bForceImmediately=False,bNotifyUserSettings=False)")
      (Transformation|AddActorLocalOffset "0, 0, 0" true false))))

(event EventTick
  (params (DeltaSeconds :type Float%20%28single-precision%29)))

(fn ConstructionScript)